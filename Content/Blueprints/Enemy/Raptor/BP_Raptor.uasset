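; Raptor enemy Blueprint that keeps its motion warping targets aligned with its current combat target.
; Each Tick, while CombatTarget is valid, it updates the TranslationTarget and RotationTarget warp targets on the MotionWarping component.
; Both targets take their location from GetTranslationWarpTarget, so rotation warps toward the same computed point as translation.
; BeginPlay, overlap and construction add no logic of their own.
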(event EventBeginPlay
  (|CallParentFunction) ; This node is disabled and will not be called.\nDrag off pins to build functionality.
)

(event Collision|EventActorBeginOverlap
  (params (OtherActor :type Actor%20Object%20Reference))
  (|CallParentFunction OtherActor) ; This node is disabled and will not be called.\nDrag off pins to build functionality.
)

(event EventTick
  (params (DeltaSeconds :type Float%20%28single-precision%29))
  (Variables|Default|GetCombatTarget
    (:then
      (bind _returnvalue (Class|BaseCharacter|GetTranslationWarpTarget))
      (Class|MotionWarpingComponent|AddorUpdateWarpTargetfromLocation (Variables|Default|GetMotionWarping) "TranslationTarget" _returnvalue)
      (bind _returnvalue_2 (Class|BaseCharacter|GetTranslationWarpTarget))
      (Class|MotionWarpingComponent|AddorUpdateWarpTargetfromLocation (Variables|Default|GetMotionWarping) "RotationTarget" _returnvalue_2))
    (:else)))

(fn ConstructionScript
  (|CallParentFunction))