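; Breakable small pot actor that shatters when hit, built on a parent breakable class with a Chaos geometry collection.
; GetHit plays the pot-break sound at the impact point, then defers to the parent's hit handling.
; When the geometry collection breaks, it sets a short lifespan for cleanup and makes the capsule ignore pawns so characters can pass through the debris.
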(event OnChaosBreakEvent(GeometryCollection)
  (params (BreakEvent :type Chaos%20Break%20Event%20Structure%20%28by%20ref%29))
  (Actor|SetLifeSpan 3.0)
  (Collision|SetCollisionResponsetoChannel (Variables|Default|GetCapsule) "ECC_Pawn" "ECR_Ignore"))

(event EventBeginPlay
  (|CallParentFunction) ; This node is disabled and will not be called.\nDrag off pins to build functionality.
)

(event Collision|EventActorBeginOverlap
  (params (OtherActor :type Actor%20Object%20Reference))
  (|CallParentFunction OtherActor) ; This node is disabled and will not be called.\nDrag off pins to build functionality.
)

(event EventTick
  (params (DeltaSeconds :type Float%20%28single-precision%29))
  (|CallParentFunction DeltaSeconds) ; This node is disabled and will not be called.\nDrag off pins to build functionality.
)

(event EventGetHit
  (params (ImpactPoint :type Vector%20%28by%20ref%29 :default "0, 0, 0"))
  (Audio|PlaySoundatLocation "/Game/Audio/MetaSounds/sfx_PotBreak.sfx_PotBreak" ImpactPoint "0, 0, 0" 1.0 1.0 0.0 0 0 0 0)
  (|CallParentFunction ImpactPoint))

(fn ConstructionScript
  (|CallParentFunction))